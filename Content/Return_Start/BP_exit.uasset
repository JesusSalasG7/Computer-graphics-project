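; Exit Blueprint that opens the "Start" level when the third-person character enters its exit box while OnLight is set.
; Any overlap on a separate trigger box requests a five-second timer, with no function name set, and starts the Checkear check.
; Checkear re-polls through a short Delay until remaining time reads exactly zero, then switches the sphere to the Light material and sets OnLight.
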(event OnComponentBeginOverlap(Box)
  (params (OverlappedComponent :type Primitive%20Component%20Object%20Reference) (OtherActor :type Actor%20Object%20Reference) (OtherComp :type Primitive%20Component%20Object%20Reference) (OtherBodyIndex :type Integer) (bFromSweep :type Boolean) (SweepResult :type Hit%20Result%20Structure%20%28by%20ref%29))
  (bind _returnvalue (Utilities|Time|SetTimerbyFunctionName 0 "" 5.0))
  (Variables|Default|SetTimer%20Light _returnvalue)
  (CallFunction|Checkear))

(event OnComponentBeginOverlap(Box1)
  (params (OverlappedComponent :type Primitive%20Component%20Object%20Reference) (OtherActor :type Actor%20Object%20Reference) (OtherComp :type Primitive%20Component%20Object%20Reference) (OtherBodyIndex :type Integer) (bFromSweep :type Boolean) (SweepResult :type Hit%20Result%20Structure%20%28by%20ref%29))
  (Utilities|Casting|CastToBP_ThirdPersonCharacter OtherActor)
  (if (Variables|Default|GetOn%20Light)
    (Game|OpenLevel(byName) "Start")))

(event Custom|Checkear
  (if (== (Utilities|Time|GetTimerRemainingTimebyHandle (Variables|Default|GetTimer%20Light)) 0.0)
    (Rendering|Material|CreateDynamicMaterialInstance (Variables|Default|GetSphere) 0 "/Game/Return_Start/Light.Light" "None" :!class /Script/Engine.PrimitiveComponent)
    (Variables|Default|SetOn%20Light true)
    (else
      (Rendering|Material|CreateDynamicMaterialInstance (Variables|Default|GetSphere) 0 "/Engine/EditorLandscapeResources/AlphaBrushMaterial_Smooth.AlphaBrushMaterial_Smooth" "None" :!class /Script/Engine.PrimitiveComponent)
      (Utilities|FlowControl|Delay 0.2)
      (CallFunction|Checkear))))

(fn ConstructionScript)