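; Interactable mirror closet whose two doors swing open in opposite directions when the player interacts nearby.
; A box overlap by the FirstPersonCharacter shows the Interfaz_Interaccion prompt widget and opens a gate that lets the Interactuar event play a Timeline.
; The Timeline drives eased yaw rotations on both doors.
; Leaving the box removes all widgets, closes the gate and reverses the Timeline to shut the doors.
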(event OnComponentBeginOverlap(Box)
  (params (OverlappedComponent :type Primitive%20Component%20Object%20Reference) (OtherActor :type Actor%20Object%20Reference) (OtherComp :type Primitive%20Component%20Object%20Reference) (OtherBodyIndex :type Integer) (bFromSweep :type Boolean) (SweepResult :type Hit%20Result%20Structure%20%28by%20ref%29))
  (Utilities|Casting|CastToFirstPersonCharacter OtherActor)
  (bind _returnvalue (UserInterface|CreateWidget "/Game/Door/Interfaz_Interaccion.Interfaz_Interaccion_C"))
  (UserInterface|Viewport|AddtoViewport _returnvalue 0)
  (Utilities|FlowControl|Gate true) ; enters at Open
)

(event OnComponentEndOverlap(Box)
  (params (OverlappedComponent :type Primitive%20Component%20Object%20Reference) (OtherActor :type Actor%20Object%20Reference) (OtherComp :type Primitive%20Component%20Object%20Reference) (OtherBodyIndex :type Integer))
  (Utilities|Casting|CastToFirstPersonCharacter OtherActor)
  (Viewport|RemoveAllWidgets)
  (Utilities|FlowControl|Sequence
    (:then_0
      (Utilities|FlowControl|Gate true) ; enters at Close
    )
    (:then_1
      (bind (_direction _alpha _alpha2) (Timeline|Timeline Reverse)
        (:Update
          (Utilities|FlowControl|Sequence
            (:then_0
              (Transformation|SetRelativeRotation (Variables|Default|GetDoor1) (Math|Rotator|MakeRotator 0.0 0.0 (Math|Interpolation|Ease "EaseInOut" _alpha 2.2e+02 3.2e+02 2.0)) false false))
            (:then_1
              (Transformation|SetRelativeRotation (Variables|Default|GetDoor2) (Math|Rotator|MakeRotator 0.0 0.0 (Math|Interpolation|Ease "EaseInOut" _alpha2 2.2e+02 1.2e+02 2.0)) false false))))))))

(event Custom|Interactuar
  (Utilities|FlowControl|Gate true
    (:Exit
      (bind (_direction _alpha _alpha2) (Timeline|Timeline Play)
        (:Update
          (Utilities|FlowControl|Sequence
            (:then_0
              (Transformation|SetRelativeRotation (Variables|Default|GetDoor1) (Math|Rotator|MakeRotator 0.0 0.0 (Math|Interpolation|Ease "EaseInOut" _alpha 2.2e+02 3.2e+02 2.0)) false false))
            (:then_1
              (Transformation|SetRelativeRotation (Variables|Default|GetDoor2) (Math|Rotator|MakeRotator 0.0 0.0 (Math|Interpolation|Ease "EaseInOut" _alpha2 2.2e+02 1.2e+02 2.0)) false false))))))))

(event EventBeginPlay)

(event Collision|EventActorBeginOverlap
  (params (OtherActor :type Actor%20Object%20Reference)))

(event EventTick
  (params (DeltaSeconds :type Float%20%28single-precision%29)))

(fn ConstructionScript)