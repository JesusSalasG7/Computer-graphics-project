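; BP_Door1_Mirror is an interactable door that swings open when triggered near it and closes when the player walks away.
; Overlap of BP_ThirdPersonCharacter with the box shows a widget and opens a gate that lets the Interactuar event through.
; Interactuar plays a timeline that eases the door's yaw and disables frame collision.
; Leaving removes all widgets, closes the gate, restores frame collision and reverses the timeline.
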(event OnComponentBeginOverlap(Box)
  (params (OverlappedComponent :type Primitive%20Component%20Object%20Reference) (OtherActor :type Actor%20Object%20Reference) (OtherComp :type Primitive%20Component%20Object%20Reference) (OtherBodyIndex :type Integer) (bFromSweep :type Boolean) (SweepResult :type Hit%20Result%20Structure%20%28by%20ref%29))
  (Utilities|Casting|CastToBP_ThirdPersonCharacter OtherActor)
  (bind _returnvalue (UserInterface|CreateWidget "/Game/Door/Interfaz_Interaccion.Interfaz_Interaccion_C"))
  (UserInterface|Viewport|AddtoViewport _returnvalue 0)
  (Utilities|FlowControl|Gate true) ; enters at Open
)

(event OnComponentEndOverlap(Box)
  (params (OverlappedComponent :type Primitive%20Component%20Object%20Reference) (OtherActor :type Actor%20Object%20Reference) (OtherComp :type Primitive%20Component%20Object%20Reference) (OtherBodyIndex :type Integer))
  (Utilities|Casting|CastToBP_ThirdPersonCharacter OtherActor)
  (Viewport|RemoveAllWidgets)
  (Utilities|FlowControl|Sequence
    (:then_0
      (Utilities|FlowControl|Gate true) ; enters at Close
    )
    (:then_1
      (Collision|SetCollisionEnabled (Variables|Default|GetFrame) "QueryAndPhysics")
      (bind _alpha (Timeline|Timeline Reverse)
        (:Update
          (Transformation|SetRelativeRotation (Variables|Default|GetDoor) (Math|Rotator|MakeRotator 0.0 0.0 (Math|Interpolation|Ease "EaseInOut" _alpha 0.0 1.2e+02 2.0)) false false)
          (Collision|SetCollisionEnabled (Variables|Default|GetFrame) "NoCollision"))))))

(event Custom|Interactuar
  (Utilities|FlowControl|Gate true
    (:Exit
      (bind _alpha (Timeline|Timeline Play)
        (:Update
          (Transformation|SetRelativeRotation (Variables|Default|GetDoor) (Math|Rotator|MakeRotator 0.0 0.0 (Math|Interpolation|Ease "EaseInOut" _alpha 0.0 1.2e+02 2.0)) false false)
          (Collision|SetCollisionEnabled (Variables|Default|GetFrame) "NoCollision"))))))

(event EventBeginPlay)

(event Collision|EventActorBeginOverlap
  (params (OtherActor :type Actor%20Object%20Reference)))

(event EventTick
  (params (DeltaSeconds :type Float%20%28single-precision%29)))

(fn ConstructionScript)